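; BP_ElectricBeam is a Niagara electric beam actor that stretches from itself toward a referenced ActorBeamEnd.
; Each Tick it line-traces to that actor on Visibility and sets the local-space BeamEnd parameter to the hit actor's origin, not the impact point.
; Without a hit, the beam ends at ActorBeamEnd.
; The Fountain and SingleLoopingParticle hit emitters are enabled only while the trace hits a BP_NiagaraUE5Logo.
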(event `self.ReceiveTick`
  (params (DeltaSeconds :type "Float (single-precision)"))
  (bind _actorbeamend (`self.ActorBeamEnd`))
  (bind _returnvalue (`self.K2_GetActorLocation` _actorbeamend))
  (`/Engine/EditorBlueprintResources/StandardMacros.IsValid` _actorbeamend
    (:`Is Valid`
      ; Only spawn hit effect when hitting
      (bind (_outhit _returnvalue_2) (`KismetSystemLibrary.LineTraceSingle` (`self.K2_GetActorLocation`) _returnvalue "TraceTypeQuery1"))
      (if _returnvalue_2
        (bind (_bblockinghit _binitialoverlap _time _distance _location _impactpoint _normal _impactnormal _physmat _hitactor) (`GameplayStatics.BreakHitResult` _outhit))
        (cast `/Game/VFX/Blueprint/BP_NiagaraUE5Logo` _hitactor
          (:`then`
            (`self.SetHitEmitters` true))
          (:`CastFailed`
            (`self.SetHitEmitters` false)))
        (`self.SetBeamEndLocation` (`self.K2_GetActorLocation` _hitactor))
        (else
          (`self.SetBeamEndLocation` _returnvalue)
          (`self.SetHitEmitters` false))))))

(fn `SetBeamEndLocation`
  (params (`World Location` :type "Vector Structure"))
  (`NiagaraComponent.SetVariableVec3` (`self.Niagara`) "BeamEnd" (`KismetMathLibrary.InverseTransformLocation` (`self.GetTransform`) `World Location`)))

(fn `SetHitEmitters`
  (params (Enable :type Boolean))
  (`FXSystemComponent.SetEmitterEnable` (`self.Niagara`) "Fountain" Enable)
  (`FXSystemComponent.SetEmitterEnable` (`self.Niagara`) "SingleLoopingParticle" Enable))

(fn `UserConstructionScript`)